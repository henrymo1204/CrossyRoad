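; BP_River is a river actor that keeps a supply of floating logs and river segments by replacing them as they reach its trigger volumes.
; BeginPlay spawns three BP_RiverSpawner segments spaced along Y, then spawns a first BP_Log after a random delay.
; A log entering Triggerzone is destroyed and replaced at SpawnPoint.
; A BP_RiverSpawner entering Box is likewise destroyed, with a replacement spawned at an offset from Scene1.
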(event `self.ReceiveBeginPlay`
  (`self.SpawnRiverAtBegin` (`self.Scene`))
  (`KismetSystemLibrary.Delay` (`KismetMathLibrary.RandomFloatInRange` 0.0 5.0))
  (`self.Spawn Log at Spawn Location` (`self.SpawnPoint`)))

(event `self.Triggerzone.OnComponentBeginOverlap`
  (params (OverlappedComponent :type "PrimitiveComponent Object Reference") (OtherActor :type "Actor Object Reference") (OtherComp :type "PrimitiveComponent Object Reference") (OtherBodyIndex :type Integer) (bFromSweep :type Boolean) (SweepResult :type "HitResult Structure (by ref)"))
  (bind _asbp_log (cast `/Game/Blueprints/BP_Log` OtherActor))
  (`self.Spawn Log at Spawn Location` (`self.SpawnPoint`))
  (`self.K2_DestroyActor` _asbp_log))

(event `self.Box.OnComponentBeginOverlap`
  (params (OverlappedComponent :type "PrimitiveComponent Object Reference") (OtherActor :type "Actor Object Reference") (OtherComp :type "PrimitiveComponent Object Reference") (OtherBodyIndex :type Integer) (bFromSweep :type Boolean) (SweepResult :type "HitResult Structure (by ref)"))
  (bind _asbp_river_spawner (cast `/Game/Blueprints/BP_RiverSpawner` OtherActor))
  (`self.SpawnRiver` (`self.Scene1`))
  (`self.K2_DestroyActor` _asbp_river_spawner))

(fn `Spawn Log at Spawn Location`
  (params (`Spawn Point` :type "SceneComponent Object Reference"))
  (`self.SpawnLog` (`SceneComponent.K2_GetComponentLocation` `Spawn Point`)))

(fn `SpawnLog`
  (params (SpawnLocation :type "Vector Structure"))
  (`|SpawnActorFromClass` "/Game/Blueprints/BP_Log.BP_Log_C" (`KismetMathLibrary.MakeTransform` SpawnLocation) "Undefined" "OverrideRootScale" null null))

(fn `SpawnRiver`
  (params (SpawnLocation :type "SceneComponent Object Reference"))
  (`|SpawnActorFromClass` "/Game/Blueprints/BP_RiverSpawner.BP_RiverSpawner_C" (`KismetMathLibrary.MakeTransform` (+ (`SceneComponent.K2_GetComponentLocation` SpawnLocation) (0.0 -1100.0 0.0))) "Undefined" "OverrideRootScale" null null))

(fn `SpawnRiverAtBegin`
  (params (SpawnLocation :type "SceneComponent Object Reference"))
  (bind _returnvalue (`SceneComponent.K2_GetComponentLocation` SpawnLocation))
  (`|SpawnActorFromClass` "/Game/Blueprints/BP_RiverSpawner.BP_RiverSpawner_C" (`KismetMathLibrary.MakeTransform` _returnvalue) "Undefined" "OverrideRootScale" null null)
  (`|SpawnActorFromClass` "/Game/Blueprints/BP_RiverSpawner.BP_RiverSpawner_C" (`KismetMathLibrary.MakeTransform` (+ _returnvalue (0.0 2200.0 0.0))) "Undefined" "OverrideRootScale" null null)
  (`|SpawnActorFromClass` "/Game/Blueprints/BP_RiverSpawner.BP_RiverSpawner_C" (`KismetMathLibrary.MakeTransform` (+ _returnvalue (0.0 -2200.0 0.0))) "Undefined" "OverrideRootScale" null null))

(fn `UserConstructionScript`)