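; BP_RiverSpawner1 is a moving river hazard that kills the player on contact; despite its name, it spawns no other actors.
; Each tick it moves along world Y by MoveSpeed scaled by delta time, with sweep enabled.
; When its static mesh hits a BP_Player1, it flags the player dead, zeroes the character model scale and plays a splash particle and sound.
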(event `self.ReceiveTick`
  (params (DeltaSeconds :type "Float (single-precision)"))
  (`self.K2_AddActorWorldOffset` (`KismetMathLibrary.MakeVector` 0.0 (* DeltaSeconds (`self.MoveSpeed`))) true))

(event `self.StaticMesh.OnComponentHit`
  (params (HitComponent :type "PrimitiveComponent Object Reference") (OtherActor :type "Actor Object Reference") (OtherComp :type "PrimitiveComponent Object Reference") (NormalImpulse :type "Vector Structure") (Hit :type "HitResult Structure (by ref)"))
  (bind _asbp_player_1 (cast `/Game/Blueprints/BP_Player1` OtherActor))
  (set `/Game/Blueprints/BP_Player1.isDead` true _asbp_player_1)
  (set `/Game/Blueprints/BP_Player1.CharacterModelScale` (0.0 0.0 0.0) _asbp_player_1)
  (bind _returnvalue (`self.K2_GetActorLocation` _asbp_player_1))
  (`self.K2_SetActorLocation` _asbp_player_1 _returnvalue false false)
  (`GameplayStatics.SpawnEmitterAtLocation` "/Game/ParticleSystem/Splash.Splash" _returnvalue)
  (`GameplayStatics.PlaySound2D` "/Game/Audio/splash_Cue.splash_Cue" 1.0 1.0 0.0 null null))

(fn `UserConstructionScript`)