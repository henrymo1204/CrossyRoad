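; BP_Player is a player Blueprint that can move until an overlap on its mesh kills it.
; While alive, Tick consumes the movement input vector and applies it as a swept local offset, without scaling by delta time.
; An overlap flattens the StaticMesh and sets IsDead, stopping movement.
; The MoveForward and MoveRight axis events are unwired, so their MaxSpeed-scaled AddMovementInput nodes never run.
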(event `InputAxis|MoveForward`
  (params (AxisValue :type "Float (single-precision)")))

(event `InputAxis|MoveRight`
  (params (AxisValue :type "Float (single-precision)")))

(event `self.ReceiveTick`
  (params (DeltaSeconds :type "Float (single-precision)"))
  (if (not (`self.isDead`))
    (bind _returnvalue (`self.ConsumeMovementInputVector`))
    (`self.K2_AddActorLocalOffset` _returnvalue true)))

(event `self.StaticMesh.OnComponentBeginOverlap`
  (params (OverlappedComponent :type "PrimitiveComponent Object Reference") (OtherActor :type "Actor Object Reference") (OtherComp :type "PrimitiveComponent Object Reference") (OtherBodyIndex :type Integer) (bFromSweep :type Boolean) (SweepResult :type "HitResult Structure (by ref)"))
  (`SceneComponent.SetRelativeScale3D` (`self.StaticMesh`) (1.0 1.0 0.001))
  (set `self.isDead` true))

(fn `UserConstructionScript`)