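; BP_Car1 is a moving car hazard that kills BP_Player1 on contact.
; It picks a random speed at BeginPlay and sweeps along negative world Y every tick.
; A blocking hit marks the player dead and squashes its model scale on X.
; An overlap also kills, but disables player collision, flattens the model on Z and moves the player to a fixed height.
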(event `self.ReceiveBeginPlay`
  (set `self.ForwardSpeed` (`KismetMathLibrary.RandomFloatInRange` -300.0 -500.0)))

(event `self.ReceiveTick`
  (params (DeltaSeconds :type "Float (single-precision)"))
  (`self.K2_AddActorWorldOffset` (`KismetMathLibrary.MakeVector` 0.0 (* DeltaSeconds (`self.ForwardSpeed`))) true))

(event `self.Car.OnComponentHit`
  (params (HitComponent :type "PrimitiveComponent Object Reference") (OtherActor :type "Actor Object Reference") (OtherComp :type "PrimitiveComponent Object Reference") (NormalImpulse :type "Vector Structure") (Hit :type "HitResult Structure (by ref)"))
  (bind _asbp_player_1 (cast `/Game/Blueprints/BP_Player1` OtherActor))
  (set `/Game/Blueprints/BP_Player1.isDead` true _asbp_player_1)
  (set `/Game/Blueprints/BP_Player1.CharacterModelScale` (0.001 1.0 1.0) _asbp_player_1)
  (`self.K2_SetActorLocation` _asbp_player_1 (`self.K2_GetActorLocation` _asbp_player_1) false false))

(event `self.Car.OnComponentBeginOverlap`
  (params (OverlappedComponent :type "PrimitiveComponent Object Reference") (OtherActor :type "Actor Object Reference") (OtherComp :type "PrimitiveComponent Object Reference") (OtherBodyIndex :type Integer) (bFromSweep :type Boolean) (SweepResult :type "HitResult Structure (by ref)"))
  (bind _asbp_player_1 (cast `/Game/Blueprints/BP_Player1` OtherActor))
  (`self.SetActorEnableCollision` _asbp_player_1 false)
  (set `/Game/Blueprints/BP_Player1.isDead` true _asbp_player_1)
  (set `/Game/Blueprints/BP_Player1.CharacterModelScale` (1.0 1.0 0.001) _asbp_player_1)
  (bind (_returnvalue_x _returnvalue_y) (`KismetMathLibrary.BreakVector` (`self.K2_GetActorLocation` _asbp_player_1)))
  (`self.K2_SetActorLocation` _asbp_player_1 (`KismetMathLibrary.MakeVector` _returnvalue_x _returnvalue_y 90.0) true false))

(fn `UserConstructionScript`)