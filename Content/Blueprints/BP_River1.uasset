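; BP_River1 is a river lane that keeps spawning logs, lilypads and river pieces.
; BeginPlay spawns three BP_RiverSpawner1 pieces along Y, then after a random delay spawns a random log or lilypad at SpawnPoint.
; Trigger zones destroy arriving logs or lilypads and spawn a random replacement, keeping the cycle going.
; A box destroys overlapping river pieces and spawns a new one at a Y offset from Scene1.
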(event `self.ReceiveBeginPlay`
  (bind _spawnpoint (`self.SpawnPoint`))
  (`self.SpawnRiverAtBegin` (`self.Scene`))
  (`KismetSystemLibrary.Delay` (`KismetMathLibrary.RandomFloatInRange` 0.0 5.0))
  (switch `int` (`KismetMathLibrary.RandomIntegerInRange` 0 1)
    (:`0`
      (`self.Spawn Log at Spawn Location` _spawnpoint))
    (:`1`
      (`self.SpawnLilypad` _spawnpoint))))

(event `self.Triggerzone.OnComponentBeginOverlap`
  (params (OverlappedComponent :type "PrimitiveComponent Object Reference") (OtherActor :type "Actor Object Reference") (OtherComp :type "PrimitiveComponent Object Reference") (OtherBodyIndex :type Integer) (bFromSweep :type Boolean) (SweepResult :type "HitResult Structure (by ref)"))
  (bind _spawnpoint (`self.SpawnPoint`))
  (bind _asbp_log_1 (cast `/Game/Blueprints/BP_Log1` OtherActor))
  (`self.K2_DestroyActor` _asbp_log_1)
  (switch `int` (`KismetMathLibrary.RandomIntegerInRange` 0 1)
    (:`0`
      (`self.Spawn Log at Spawn Location` _spawnpoint))
    (:`1`
      (`self.SpawnLilypad` _spawnpoint))))

(event `self.Triggerzone1.OnComponentBeginOverlap`
  (params (OverlappedComponent :type "PrimitiveComponent Object Reference") (OtherActor :type "Actor Object Reference") (OtherComp :type "PrimitiveComponent Object Reference") (OtherBodyIndex :type Integer) (bFromSweep :type Boolean) (SweepResult :type "HitResult Structure (by ref)"))
  (bind _spawnpoint (`self.SpawnPoint`))
  (bind _asbp_lilypad_1 (cast `/Game/Blueprints/BP_Lilypad1` OtherActor))
  (`self.K2_DestroyActor` _asbp_lilypad_1)
  (switch `int` (`KismetMathLibrary.RandomIntegerInRange` 0 1)
    (:`0`
      (`self.Spawn Log at Spawn Location` _spawnpoint))
    (:`1`
      (`self.SpawnLilypad` _spawnpoint))))

(event `self.Box.OnComponentBeginOverlap`
  (params (OverlappedComponent :type "PrimitiveComponent Object Reference") (OtherActor :type "Actor Object Reference") (OtherComp :type "PrimitiveComponent Object Reference") (OtherBodyIndex :type Integer) (bFromSweep :type Boolean) (SweepResult :type "HitResult Structure (by ref)"))
  (bind _asbp_river_spawner_1 (cast `/Game/Blueprints/BP_RiverSpawner1` OtherActor))
  (`self.SpawnRiver` (`self.Scene1`))
  (`self.K2_DestroyActor` _asbp_river_spawner_1))

(fn `Spawn Log at Spawn Location`
  (params (`Spawn Point` :type "SceneComponent Object Reference"))
  (`self.SpawnLog` (`SceneComponent.K2_GetComponentLocation` `Spawn Point`)))

(fn `SpawnLilypad`
  (params (SpawnLocation :type "SceneComponent Object Reference"))
  (`|SpawnActorFromClass` "/Game/Blueprints/BP_Lilypad1.BP_Lilypad1_C" (`KismetMathLibrary.MakeTransform` (`SceneComponent.K2_GetComponentLocation` SpawnLocation)) "Undefined" "OverrideRootScale" null null))

(fn `SpawnLog`
  (params (SpawnLocation :type "Vector Structure"))
  (`|SpawnActorFromClass` "/Game/Blueprints/BP_Log1.BP_Log1_C" (`KismetMathLibrary.MakeTransform` SpawnLocation) "Undefined" "OverrideRootScale" null null))

(fn `SpawnRiver`
  (params (SpawnLocation :type "SceneComponent Object Reference"))
  (`|SpawnActorFromClass` "/Game/Blueprints/BP_RiverSpawner1.BP_RiverSpawner1_C" (`KismetMathLibrary.MakeTransform` (+ (`SceneComponent.K2_GetComponentLocation` SpawnLocation) (0.0 1100.0 0.0))) "Undefined" "OverrideRootScale" null null))

(fn `SpawnRiverAtBegin`
  (params (SpawnLocation :type "SceneComponent Object Reference"))
  (bind _returnvalue (`SceneComponent.K2_GetComponentLocation` SpawnLocation))
  (`|SpawnActorFromClass` "/Game/Blueprints/BP_RiverSpawner1.BP_RiverSpawner1_C" (`KismetMathLibrary.MakeTransform` _returnvalue) "Undefined" "OverrideRootScale" null null)
  (`|SpawnActorFromClass` "/Game/Blueprints/BP_RiverSpawner1.BP_RiverSpawner1_C" (`KismetMathLibrary.MakeTransform` (+ _returnvalue (0.0 2200.0 0.0))) "Undefined" "OverrideRootScale" null null)
  (`|SpawnActorFromClass` "/Game/Blueprints/BP_RiverSpawner1.BP_RiverSpawner1_C" (`KismetMathLibrary.MakeTransform` (+ _returnvalue (0.0 -2200.0 0.0))) "Undefined" "OverrideRootScale" null null))

(fn `UserConstructionScript`)