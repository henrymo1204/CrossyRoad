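; Endless lane-based map spawner that generates random road, railroad, river and grass strips along +X.
; BeginPlay lays alternating starter grass, then runs SpawnMap, which places random strips at an advancing SpawnPoint and moves TriggerZone to mid-batch.
; BP_Player1 overlapping the actor spawns the next batch.
; IsHighway tracks road runs to insert markings between roads and a BP_Highway closing piece, while IsGrass0 alternates the grass variants.
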(event `self.ReceiveBeginPlay`
  (bind _spawnpoint (`self.SpawnPoint`))
  (for _ (range 5)
    (if (`self.isGrass0`)
      (`self.SpawnGrass0` _spawnpoint)
      (set `self.isGrass0` false)
      (else
        (`self.SpawnGrass1` _spawnpoint)
        (set `self.isGrass0` true)))
    (`SceneComponent.K2_SetWorldLocation` (`self.SpawnPoint`) (+ (`SceneComponent.K2_GetComponentLocation` _spawnpoint) (80.0 0.0 0.0)) false false))
  (`self.Spawn Map` :!label _label))

(event `self.ReceiveActorBeginOverlap`
  (params (OtherActor :type "Actor Object Reference"))
  (cast `/Game/Blueprints/BP_Player1` OtherActor)
  (goto _label))

(fn `Spawn Map`
  (bind _spawnpoint (`self.SpawnPoint`))
  (bind _returnvalue (`SceneComponent.K2_GetComponentLocation` _spawnpoint))
  (bind _returnvalue_2 (+ (`SceneComponent.K2_GetComponentLocation` _spawnpoint) (40.0 0.0 0.0)))
  (for _index (range 16)
    (if (== _index 7)
      (`SceneComponent.K2_SetWorldLocation` (`self.TriggerZone`) _returnvalue false false)
      (else
        (switch `int` (`KismetMathLibrary.RandomIntegerInRange` 0 3)
          (:`0`
            (if (`self.isHighway`)
              (`self.SpawnMarking` _spawnpoint)
              (`SceneComponent.K2_SetWorldLocation` (`self.SpawnPoint`) (+ (`SceneComponent.K2_GetComponentLocation` _spawnpoint) (40.0 0.0 0.0)) true false))
            (`self.SpawnRoad` _spawnpoint)
            (set `self.isHighway` true)
            (`SceneComponent.K2_SetWorldLocation` (`self.SpawnPoint`) (+ _returnvalue (40.0 0.0 0.0)) true false))
          (:`1`
            (if (`self.isHighway`)
              (`self.SpawnHighway` _spawnpoint)
              (`SceneComponent.K2_SetWorldLocation` (`self.SpawnPoint`) _returnvalue_2 true false)
              (set `self.isHighway` false))
            (`self.SpawnRailroad` _spawnpoint)
            (`SceneComponent.K2_SetWorldLocation` (`self.SpawnPoint`) (+ _returnvalue (80.0 0.0 0.0)) true false :!label _label))
          (:`2`
            (if (`self.isHighway`)
              (`self.SpawnHighway` _spawnpoint)
              (`SceneComponent.K2_SetWorldLocation` (`self.SpawnPoint`) _returnvalue_2 true false)
              (set `self.isHighway` false))
            (`self.SpawnRiver` _spawnpoint)
            (goto _label))
          (:`3`
            (if (`self.isHighway`)
              (`self.SpawnHighway` _spawnpoint)
              (`SceneComponent.K2_SetWorldLocation` (`self.SpawnPoint`) _returnvalue_2 true false)
              (set `self.isHighway` false))
            (if (`self.isGrass0`)
              (`self.SpawnGrass0` _spawnpoint)
              (set `self.isGrass0` false)
              (goto _label)
              (else
                (`self.SpawnGrass1` _spawnpoint)
                (set `self.isGrass0` true)
                (goto _label)))))))))

(fn `SpawnGrass0`
  (params (SpawnLocation :type "SceneComponent Object Reference"))
  (`|SpawnActorFromClass` "/Game/Blueprints/BP_Grass0.BP_Grass0_C" (`KismetMathLibrary.MakeTransform` (`SceneComponent.K2_GetComponentLocation` SpawnLocation)) "Undefined" "OverrideRootScale" null null))

(fn `SpawnGrass1`
  (params (SpawnLocation :type "SceneComponent Object Reference"))
  (`|SpawnActorFromClass` "/Game/Blueprints/BP_Grass1.BP_Grass1_C" (`KismetMathLibrary.MakeTransform` (`SceneComponent.K2_GetComponentLocation` SpawnLocation)) "Undefined" "OverrideRootScale" null null))

(fn `SpawnHighway`
  (params (SpawnLocation :type "SceneComponent Object Reference"))
  (`|SpawnActorFromClass` "/Game/Blueprints/BP_Highway.BP_Highway_C" (`KismetMathLibrary.MakeTransform` (`SceneComponent.K2_GetComponentLocation` SpawnLocation)) "Undefined" "OverrideRootScale" null null))

(fn `SpawnMarking`
  (params (SpawnLocation :type "SceneComponent Object Reference"))
  (`|SpawnActorFromClass` "/Game/Blueprints/BP_Marking.BP_Marking_C" (`KismetMathLibrary.MakeTransform` (`SceneComponent.K2_GetComponentLocation` SpawnLocation)) "Undefined" "OverrideRootScale" null null))

(fn `SpawnRailroad`
  (params (SpawnLocation :type "SceneComponent Object Reference"))
  (`|SpawnActorFromClass` "/Game/Blueprints/BP_Railroad.BP_Railroad_C" (`KismetMathLibrary.MakeTransform` (`SceneComponent.K2_GetComponentLocation` SpawnLocation)) "Undefined" "OverrideRootScale" null null))

(fn `SpawnRiver`
  (params (SpawnLocation :type "SceneComponent Object Reference"))
  (`|SpawnActorFromClass` "/Game/Blueprints/BP_River.BP_River_C" (`KismetMathLibrary.MakeTransform` (`SceneComponent.K2_GetComponentLocation` SpawnLocation)) "Undefined" "OverrideRootScale" null null))

(fn `SpawnRoad`
  (params (SpawnLocation :type "SceneComponent Object Reference"))
  (`|SpawnActorFromClass` "/Game/Blueprints/BP_Road0.BP_Road0_C" (`KismetMathLibrary.MakeTransform` (`SceneComponent.K2_GetComponentLocation` SpawnLocation)) "Undefined" "OverrideRootScale" null null))

(fn `UserConstructionScript`)