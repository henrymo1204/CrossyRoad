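; BP_Road is a road actor that keeps a continuous stream of BP_Car traffic in the level.
; On BeginPlay it spawns an evenly spaced row of cars along X at hard-coded world positions.
; Two trigger zones recycle traffic: an overlapping car is destroyed and a fresh one is spawned at that zone's paired spawn point, through shared spawn helper functions.
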(event `self.ReceiveBeginPlay`
  (for _index (range 13)
    (`self.SpawnCar` (`KismetMathLibrary.MakeVector` (+ (* (`KismetMathLibrary.Conv_IntToDouble` _index) 80.0) -400.0) -470.0))))

(event `self.TriggerZone1.OnComponentBeginOverlap`
  (params (OverlappedComponent :type "PrimitiveComponent Object Reference") (OtherActor :type "Actor Object Reference") (OtherComp :type "PrimitiveComponent Object Reference") (OtherBodyIndex :type Integer) (bFromSweep :type Boolean) (SweepResult :type "HitResult Structure (by ref)"))
  (bind _asbp_car (cast `/Game/Blueprints/BP_Car` OtherActor))
  (`self.Spawn Car at Spawn Point` (`self.SpawnPoint1`))
  (`self.K2_DestroyActor` _asbp_car))

(event `self.TriggerZone2.OnComponentBeginOverlap`
  (params (OverlappedComponent :type "PrimitiveComponent Object Reference") (OtherActor :type "Actor Object Reference") (OtherComp :type "PrimitiveComponent Object Reference") (OtherBodyIndex :type Integer) (bFromSweep :type Boolean) (SweepResult :type "HitResult Structure (by ref)"))
  (bind _asbp_car (cast `/Game/Blueprints/BP_Car` OtherActor))
  (`self.Spawn Car at Spawn Point` (`self.SpawnPoint2`))
  (`self.K2_DestroyActor` _asbp_car))

(fn `Spawn Car at Spawn Point`
  (params (SpawnPoint :type "SceneComponent Object Reference"))
  (`self.SpawnCar` (`SceneComponent.K2_GetComponentLocation` SpawnPoint)))

(fn `SpawnCar`
  (params (SpawnLocation :type "Vector Structure"))
  (`|SpawnActorFromClass` "/Game/Blueprints/BP_Car.BP_Car_C" (`KismetMathLibrary.MakeTransform` SpawnLocation) "Undefined" "OverrideRootScale" null null))

(fn `UserConstructionScript`)