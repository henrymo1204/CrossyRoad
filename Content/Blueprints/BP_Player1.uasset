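; Player character for a hop-based, car-dodging game in the style of Frogger.
; Four move inputs launch it in fixed world-axis arcs, turn the mesh via a stored facing index (left and right switch on a constant instead), and play a hop sound.
; Each hop disables input until Tick finds it no longer falling.
; Overlapping BP_Car kills it: collision turns off, height is fixed, and Tick applies the death mesh scale.
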(event `InputAction|MoveForward`
  (params (Key :type "Key Structure"))
  (:`Pressed`
    (if (not (`self.isDead`))
      (switch `int` (`self.current`)
        (:`0`
          _)
        (:`1`
          (`SceneComponent.K2_SetWorldRotation` :`self` (`self.StaticMesh`) :!label _label))
        (:`2`
          (goto _label))
        (:`3`
          (goto _label)))
      (`self.LaunchCharacter` (160.0 0.0 200.0) true true)
      (`GameplayStatics.PlaySound2D` "/Game/Audio/Hop_Cue.Hop_Cue" 1.0 1.0 0.0 null null)
      (`self.DisableInput` null)
      (set `self.current` 0))))

(event `InputAction|MoveBackward`
  (params (Key :type "Key Structure"))
  (:`Pressed`
    (if (not (`self.isDead`))
      (switch `int` (`self.current`)
        (:`0`
          (`SceneComponent.K2_SetWorldRotation` (`self.StaticMesh`) (struct :`Yaw` 180.0) false false :!label _label_2))
        (:`1`
          (goto _label_2))
        (:`2`
          _)
        (:`3`
          (goto _label_2)))
      (`self.LaunchCharacter` (-160.0 0.0 200.0) true true)
      (`GameplayStatics.PlaySound2D` "/Game/Audio/Hop_Cue.Hop_Cue" 1.0 1.0 0.0 null null)
      (`self.DisableInput` null)
      (set `self.current` 2))))

(event `InputAction|MoveRight`
  (params (Key :type "Key Structure"))
  (:`Pressed`
    (if (not (`self.isDead`))
      (switch `int` 0
        (:`0`
          (`SceneComponent.K2_SetWorldRotation` (`self.StaticMesh`) (struct :`Yaw` 90.0) false false :!label _label_3))
        (:`1`
          (goto _label_3))
        (:`2`
          _)
        (:`3`
          (goto _label_3)))
      (`self.LaunchCharacter` (0.0 120.0 200.0) true true)
      (`GameplayStatics.PlaySound2D` "/Game/Audio/Hop_Cue.Hop_Cue" 1.0 1.0 0.0 null null)
      (`self.DisableInput` null)
      (set `self.current` 1))))

(event `InputAction|MoveLeft`
  (params (Key :type "Key Structure"))
  (:`Pressed`
    (if (not (`self.isDead`))
      (switch `int` 0
        (:`0`
          (`SceneComponent.K2_SetWorldRotation` (`self.StaticMesh`) (struct :`Yaw` 270.0) false false :!label _label_4))
        (:`1`
          (goto _label_4))
        (:`2`
          _)
        (:`3`
          (goto _label_4)))
      (`self.LaunchCharacter` (0.0 -120.0 200.0) true true)
      (`GameplayStatics.PlaySound2D` "/Game/Audio/Hop_Cue.Hop_Cue" 1.0 1.0 0.0 null null)
      (`self.DisableInput` null)
      (set `self.current` 3))))

(event `self.ReceiveTick`
  (params (DeltaSeconds :type "Float (single-precision)"))
  (if (`self.isDead`)
    (`SceneComponent.SetRelativeScale3D` (`self.StaticMesh`) (`self.CharacterModelScale`))
    (elif (not (`NavMovementComponent.IsFalling` (`self.CharacterMovement`)))
      (`self.EnableInput` null))))

(event `self.ReceiveActorBeginOverlap`
  (params (OtherActor :type "Actor Object Reference"))
  (bind (_returnvalue_x _returnvalue_y) (`KismetMathLibrary.BreakVector` (`self.K2_GetActorLocation`)))
  (cast `/Game/Blueprints/BP_Car` OtherActor)
  (`self.SetActorEnableCollision` false)
  (set `self.isDead` true)
  (`self.K2_SetActorLocation` (`KismetMathLibrary.MakeVector` _returnvalue_x _returnvalue_y 90.0) true))

(fn `UserConstructionScript`)