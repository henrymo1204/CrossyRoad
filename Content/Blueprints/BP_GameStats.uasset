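; Game stats actor that tracks the current and high score and drives their display on the HUD.
; BeginPlay creates WBP_Hud, hands it a self-reference and stores it in two variables, HUDWidget and Hudwid.
; Each Tick refreshes both HUD texts, then reads TotalScore from the first BP_Player1 found via GetAllActorsOfClass, raising HighScore when beaten.
; HighScore is not saved here, and the HUD refresh precedes each score update.
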(event `self.ReceiveBeginPlay`
  (bind _returnvalue (`|CreateWidget` "/Game/UI/WBP_Hud.WBP_Hud_C"))
  (`UserWidget.AddToViewport` _returnvalue 0)
  (set `/Game/UI/WBP_Hud.GameStatss` self _returnvalue)
  (bind _output_get (set `self.HUDWidget` _returnvalue))
  (`/Game/UI/WBP_Hud.updateScoreText` _output_get)
  (bind _output_get_2 (set `self.hudwid` _returnvalue))
  (`/Game/UI/WBP_Hud.updateHighScoreText` _output_get_2))

(event `self.ReceiveTick`
  (params (DeltaSeconds :type "Float (single-precision)"))
  (bind _outactors (`GameplayStatics.GetAllActorsOfClass` "/Game/Blueprints/BP_Player1.BP_Player1_C"))
  (`self.incrementScoreCollected`)
  (bind _output_get (set `self.currentScore` (`/Game/Blueprints/BP_Player1.TotalScore` (`|GetArrayItem` _outactors))))
  (if (> _output_get (`self.highScore`))
    (set `self.highScore` _output_get)))

(fn `incrementScoreCollected`
  (`/Game/UI/WBP_Hud.updateScoreText` (`self.HUDWidget`))
  (`/Game/UI/WBP_Hud.updateHighScoreText` (`self.hudwid`)))

(fn `UserConstructionScript`)