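; Railroad actor that keeps spawning trains of random length and removes them when their parts hit its trigger boxes.
; SpawnTrain places a tail, zero to two bodies and a head, stepping a scene component along Y as a placement cursor, then resets it to a second scene component.
; Three boxes destroy head, body and tail respectively, and the tail's removal spawns the next train, keeping the cycle going from BeginPlay.
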(event `self.ReceiveBeginPlay`
  (`self.SpawnTrain` (`self.Scene`)))

(event `self.Box.OnComponentBeginOverlap`
  (params (OverlappedComponent :type "PrimitiveComponent Object Reference") (OtherActor :type "Actor Object Reference") (OtherComp :type "PrimitiveComponent Object Reference") (OtherBodyIndex :type Integer) (bFromSweep :type Boolean) (SweepResult :type "HitResult Structure (by ref)"))
  (bind _asbp_train (cast `/Game/Blueprints/BP_TrainHead` OtherActor))
  (`self.K2_DestroyActor` _asbp_train))

(event `self.Box1.OnComponentBeginOverlap`
  (params (OverlappedComponent :type "PrimitiveComponent Object Reference") (OtherActor :type "Actor Object Reference") (OtherComp :type "PrimitiveComponent Object Reference") (OtherBodyIndex :type Integer) (bFromSweep :type Boolean) (SweepResult :type "HitResult Structure (by ref)"))
  (bind _asbp_train_body (cast `/Game/Blueprints/BP_TrainBody` OtherActor))
  (`self.K2_DestroyActor` _asbp_train_body))

(event `self.Box2.OnComponentBeginOverlap`
  (params (OverlappedComponent :type "PrimitiveComponent Object Reference") (OtherActor :type "Actor Object Reference") (OtherComp :type "PrimitiveComponent Object Reference") (OtherBodyIndex :type Integer) (bFromSweep :type Boolean) (SweepResult :type "HitResult Structure (by ref)"))
  (bind _asbp_train_tail (cast `/Game/Blueprints/BP_TrainTail` OtherActor))
  (`self.K2_DestroyActor` _asbp_train_tail)
  (`self.SpawnTrain` (`self.Scene`)))

(fn `SpawnTrain`
  (params (SpawnLocation :type "SceneComponent Object Reference"))
  (bind _scene (`self.Scene`))
  (bind _returnvalue (`SceneComponent.K2_GetComponentLocation` (`self.Scene`)))
  (`|SpawnActorFromClass` "/Game/Blueprints/BP_TrainTail.BP_TrainTail_C" (`KismetMathLibrary.MakeTransform` (`SceneComponent.K2_GetComponentLocation` SpawnLocation) (struct)) "Undefined" "OverrideRootScale" null null)
  (`SceneComponent.K2_SetWorldLocation` _scene (+ (`SceneComponent.K2_GetComponentLocation` _scene) (0.0 370.0 0.0)) true false)
  (switch `int` (`KismetMathLibrary.RandomIntegerInRange` 0 2)
    (:`0`
      (`SceneComponent.K2_SetWorldLocation` (`self.Scene`) (+ _returnvalue (0.0 10.0 0.0)) true false :!label _label))
    (:`1`
      (`|SpawnActorFromClass` "/Game/Blueprints/BP_TrainBody.BP_TrainBody_C" (`KismetMathLibrary.MakeTransform` _returnvalue) "Undefined" "OverrideRootScale" null null)
      (`SceneComponent.K2_SetWorldLocation` (`self.Scene`) (+ _returnvalue (0.0 360.0 0.0)) true false)
      (goto _label))
    (:`2`
      (for _ (range 2)
        (`|SpawnActorFromClass` "/Game/Blueprints/BP_TrainBody.BP_TrainBody_C" (`KismetMathLibrary.MakeTransform` _returnvalue) "Undefined" "OverrideRootScale" null null)
        (`SceneComponent.K2_SetWorldLocation` (`self.Scene`) (+ _returnvalue (0.0 360.0 0.0)) true false))
      (`SceneComponent.K2_SetWorldLocation` (`self.Scene`) (+ _returnvalue (0.0 10.0 0.0)) true false)))
  (`|SpawnActorFromClass` "/Game/Blueprints/BP_TrainHead.BP_TrainHead_C" (`KismetMathLibrary.MakeTransform` _returnvalue) "Undefined" "OverrideRootScale" null null)
  (`SceneComponent.K2_SetWorldLocation` (`self.Scene`) (`SceneComponent.K2_GetComponentLocation` (`self.Scene1`)) false false))

(fn `UserConstructionScript`)